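; BP_Array is a construction-script tool that builds randomized 3D grids of instanced meshes.
; Each AssetList entry spawns a Hierarchical Instanced Static Mesh component, with instances spaced by mesh bounds plus offset along three axes.
; A per-entry seeded stream jitters location, rotation and scale within min/max ranges.
; Per-index overrides then add location and rotation and replace scale, before listed instances are removed.
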(fn `UserConstructionScript`
  (bind _stream (`self.Stream`))
  (bind (_currentdata_transfrom _currentdata_mesh _currentdata_count _currentdata_offset _currentdata_instancetransform _currentdata_removeinstance _currentdata_seed _currentdata_transformmin _currentdata_transformmax) (break `/Game/bluePrint/F_AssetData` (`self.CurrentData`)))
  (bind _currenthism (`self.CurrentHISM`))
  (bind (_x _y _z) (break `IntVector` _currentdata_count))
  (bind (_returnvalue_min _returnvalue_max) (break `Box` (`StaticMesh.GetBoundingBox` _currentdata_mesh)))
  (bind (_returnvalue_x _returnvalue_y _returnvalue_z) (`KismetMathLibrary.BreakVector` (- _returnvalue_max _returnvalue_min)))
  (bind _values (`BlueprintMapLibrary.Map_Values` (`self.AssetList`)))
  (for _array_element _values
    (bind _output_get (set `self.CurrentData` _array_element))
    (`KismetMathLibrary.SetRandomStreamSeed` (`self.Stream`) (`.seed_22_4F2F823442229F86B42F0F84AF513A70` (break `/Game/bluePrint/F_AssetData` _output_get)))
    (bind _returnvalue (`AddComponent|NODE_AddHierarchicalInstancedStaticMeshComponent-0` :`RelativeTransform` (break `/Game/bluePrint/F_AssetData` _output_get)))
    (bind _output_get_2 (set `self.CurrentHISM` _returnvalue))
    (`StaticMeshComponent.SetStaticMesh` _output_get_2 _currentdata_mesh)
    (for _index (range _x)
      (for _index_2 (range _y)
        (for _index_3 (range _z)
          (`InstancedStaticMeshComponent.AddInstance` (`self.CurrentHISM`) (`KismetMathLibrary.MakeTransform` (+ (`KismetMathLibrary.MakeVector` (* _index (+ _returnvalue_x (.x _currentdata_offset))) (* _index_2 (+ _returnvalue_y (.y _currentdata_offset))) (* _index_3 (+ _returnvalue_z (.z _currentdata_offset)))) (`KismetMathLibrary.MakeVector` (`KismetMathLibrary.RandomFloatInRangeFromStream` (.x (.location _currentdata_transformmin)) (.x (.location _currentdata_transformmax)) _stream) (`KismetMathLibrary.RandomFloatInRangeFromStream` (.y (.location _currentdata_transformmin)) (.y (.location _currentdata_transformmax)) _stream) (`KismetMathLibrary.RandomFloatInRangeFromStream` (.z (.location _currentdata_transformmin)) (.z (.location _currentdata_transformmax)) _stream))) (`KismetMathLibrary.MakeRotator` (`KismetMathLibrary.RandomFloatInRangeFromStream` (.roll (.rotation _currentdata_transformmin)) (.roll (.rotation _currentdata_transformmax)) _stream) (`KismetMathLibrary.RandomFloatInRangeFromStream` (.pitch (.rotation _currentdata_transformmin)) (.pitch (.rotation _currentdata_transformmax)) _stream) (`KismetMathLibrary.RandomFloatInRangeFromStream` (.yaw (.rotation _currentdata_transformmin)) (.yaw (.rotation _currentdata_transformmax)) _stream)) (`KismetMathLibrary.MakeVector` (`KismetMathLibrary.RandomFloatInRangeFromStream` (.x (.scale _currentdata_transformmin)) (.x (.scale _currentdata_transformmax)) _stream) (`KismetMathLibrary.RandomFloatInRangeFromStream` (.y (.scale _currentdata_transformmin)) (.y (.scale _currentdata_transformmax)) _stream) (`KismetMathLibrary.RandomFloatInRangeFromStream` (.z (.scale _currentdata_transformmin)) (.z (.scale _currentdata_transformmax)) _stream)))))))
    (for _array_element_2 _currentdata_instancetransform
      (bind (_id _transform) (break `/Game/bluePrint/F_InstanceeData` _array_element_2))
      (bind _outinstancetransform (`InstancedStaticMeshComponent.GetInstanceTransform` _currenthism _id false))
      (`InstancedStaticMeshComponent.UpdateInstanceTransform` _currenthism _id (`KismetMathLibrary.MakeTransform` (+ (.location _outinstancetransform) (.location _transform)) (`KismetMathLibrary.MakeRotator` (+ (.roll (.rotation _outinstancetransform)) (.roll (.rotation _transform))) (+ (.pitch (.rotation _outinstancetransform)) (.pitch (.rotation _transform))) (+ (.yaw (.rotation _outinstancetransform)) (.yaw (.rotation _transform)))) (.scale _transform)) false false false))
    (for _array_element_3 _currentdata_removeinstance
      (`InstancedStaticMeshComponent.RemoveInstance` (`self.CurrentHISM`) _array_element_3))))